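; Detachable, grabbable magazine for the M1911 pistol that tracks its round count and starts full.
; Every Tick it checks whether its attach parent belongs to a gun, showing a camera-facing ammo count widget only while held outside one.
; RemoveRound decrements the count and calls HasRound, which toggles two visible round components and the empty flag.
; Separate functions play insert and removal sounds at the magazine mesh.
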(event `self.ReceiveBeginPlay`
  (`SceneComponent.SetVisibility` (`self.AmmoWidget`) false false))

(event `self.ReceiveTick`
  (params (DeltaSeconds :type "Float (single-precision)"))
  (bind _ammowidget (`self.AmmoWidget`))
  (bind _returnvalue (`SceneComponent.GetAttachParent` (`self.RootComponent`)))
  (`/Engine/EditorBlueprintResources/StandardMacros.IsValid` _returnvalue
    (:`Is Valid`
      (set `self.bInGun` (`GameplayStatics.ObjectIsA` (`ActorComponent.GetOwner` _returnvalue) (`self.GunBlueprint`))))
    (:`Is Not Valid`
      (set `self.bInGun` false)))
  (if (and (`/Game/Blueprints/CurlGrabComponent.bIsHeld` (`self.CurlGrabComponent`)) (not (`self.bInGun`)))
    (`SceneComponent.K2_SetWorldRotation` _ammowidget (`KismetMathLibrary.FindLookAtRotation` (`SceneComponent.K2_GetComponentLocation` (`self.AmmoWidget`)) (`PlayerCameraManager.GetCameraLocation` (`PlayerController.PlayerCameraManager` (`GameplayStatics.GetPlayerController` 0)))) false false)
    (`SceneComponent.SetVisibility` _ammowidget true false)
    (bind _aswbp_mag_ammo (cast `/Game/Blueprints/HUD/WBP_MagAmmo` (`WidgetComponent.GetUserWidgetObject` _ammowidget)))
    (`TextBlock.SetText` (`/Game/Blueprints/HUD/WBP_MagAmmo.TXT_Rounds` _aswbp_mag_ammo) (`|FormatText` "{Current} / {Max}" (`self.Rounds`) (`self.MaxRounds`)))
    (else
      (`SceneComponent.SetVisibility` _ammowidget false false))))

(fn `HasRound`
  (bind _round (`self.Round`))
  (bind _round2 (`self.Round2`))
  (if (== (`self.Rounds`) 0)
    (`SceneComponent.SetVisibility` _round false false)
    (`SceneComponent.SetVisibility` _round2 false false)
    (set `self.IsEmpty` true)
    (else
      (`SceneComponent.SetVisibility` _round true false)
      (`SceneComponent.SetVisibility` _round2 true false)
      (set `self.IsEmpty` false)))
  (return))

(fn `PlayInSound`
  (`GameplayStatics.PlaySoundAtLocation` (`self.MagInSound`) (`SceneComponent.K2_GetComponentLocation` (`self.MagazineMesh`)) (struct) 1.0 1.0 0.0 null null null null))

(fn `PlayOutSound`
  (`GameplayStatics.PlaySoundAtLocation` (`self.MagOutSound`) (`SceneComponent.K2_GetComponentLocation` (`self.MagazineMesh`)) (struct) 1.0 1.0 0.0 null null null null))

(fn `RemoveRound`
  (`/Engine/EditorBlueprintResources/StandardMacros.DecrementInt` (`self.Rounds`)
    (:`  `
      (`self.HasRound`))))

(fn `UserConstructionScript`
  (set `self.Rounds` (`self.MaxRounds`)))