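; Shooting range paper target that slides back and forth along the Y axis and shows bullet holes where it is hit.
; BeginPlay gives each target its own render target, binds it to the paper mesh's dynamic material, and randomizes the starting position.
; Draw takes a 2D location and paints the bullet-hole material into that render target.
; Tick moves the target at MoveSpeed within fixed bounds, flipping direction at each end.
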(event `self.ReceiveBeginPlay`
  (bind (_returnvalue_x _returnvalue_y _returnvalue_z) (`KismetMathLibrary.BreakVector` (`self.K2_GetActorLocation`)))
  (`|ExecutionSequence`
    (:`then_0`
      (bind _returnvalue (`PrimitiveComponent.CreateDynamicMaterialInstance` (`self.TargetPaper_Skeletal`) 0 "/Game/FABS/Indoor_Shooting_Range/Materials/Target_M.Target_M" "None"))
      (bind _returnvalue_2 (`KismetMaterialLibrary.CreateDynamicMaterialInstance` "/Game/FABS/Indoor_Shooting_Range/Materials/BolletHole_M.BolletHole_M"))
      (set `self.DrawLocation` _returnvalue_2)
      (bind _returnvalue_3 (`CanvasRenderTarget2D.CreateCanvasRenderTarget2D` "/Script/Engine.CanvasRenderTarget2D" 512 768))
      (set `self.UniqueRenderT` _returnvalue_3)
      (`MaterialInstanceDynamic.SetTextureParameterValue` _returnvalue "RenderT" (`self.UniqueRenderT`))
      (`KismetRenderingLibrary.ClearRenderTarget2D` (`self.UniqueRenderT`)))
    (:`then_1`
      ;[1 1 1] Spawn Actor
      (`self.K2_SetActorLocation` (`KismetMathLibrary.MakeVector` _returnvalue_x (`KismetMathLibrary.RandomFloatInRange` 840.0 1555.0) _returnvalue_z)))))

(event `Draw`
  (params (Vector2D :type "Vector2D Structure"))
  (bind _drawlocation (`self.DrawLocation`))
  (`MaterialInstanceDynamic.SetVectorParameterValue` _drawlocation "Location" (`KismetMathLibrary.Conv_VectorToLinearColor` (`KismetMathLibrary.Conv_Vector2DToVector` Vector2D)))
  (`KismetRenderingLibrary.DrawMaterialToRenderTarget` (`self.UniqueRenderT`) _drawlocation))

(event `self.ReceiveTick`
  (params (DeltaSeconds :type "Float (single-precision)"))
  (bind (_returnvalue_x _returnvalue_y _returnvalue_z) (`KismetMathLibrary.BreakVector` (`self.K2_GetActorLocation`)))
  ;[1 1 1] Target Movement
  (`|ExecutionSequence`
    (:`then_0`
      (`self.K2_SetActorLocation` (`KismetMathLibrary.MakeVector` _returnvalue_x (`KismetMathLibrary.FClamp` (+ _returnvalue_y (* DeltaSeconds (`self.Move Direction`) (`self.MoveSpeed`))) 840.0 1555.0) _returnvalue_z)))
    (:`then_1`
      (if (>= _returnvalue_y 1555.0)
        (set `self.Move Direction` -1)))
    (:`then_2`
      (if (<= _returnvalue_y 840.0)
        (set `self.Move Direction` 1)))))

(fn `UserConstructionScript`)