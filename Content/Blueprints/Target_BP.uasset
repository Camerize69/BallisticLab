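; Shooting range paper target that slides back and forth along world Y between fixed limits and tallies hits and score.
; On BeginPlay it feeds a per-instance render target into the paper's material, and Draw stamps bullet holes onto it at a given 2D location.
; Head and body shot events add different scores.
; ActivateTarget randomizes position and direction and scales speed by a multiplier; DeactivateAndResetTarget stops and re-parks it.
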(event `self.ReceiveBeginPlay`
  (`|ExecutionSequence`
    (:`then_0`
      (bind _returnvalue (`PrimitiveComponent.CreateDynamicMaterialInstance` (`self.TargetPaper_Skeletal`) 0 "/Game/FABS/Indoor_Shooting_Range/Materials/Target_M.Target_M" "None"))
      (bind _returnvalue_2 (`KismetMaterialLibrary.CreateDynamicMaterialInstance` "/Game/FABS/Indoor_Shooting_Range/Materials/BolletHole_M.BolletHole_M"))
      (set `self.DrawLocation` _returnvalue_2)
      (bind _returnvalue_3 (`CanvasRenderTarget2D.CreateCanvasRenderTarget2D` "/Script/Engine.CanvasRenderTarget2D" 512 768))
      (set `self.UniqueRenderT` _returnvalue_3)
      (`MaterialInstanceDynamic.SetTextureParameterValue` _returnvalue "RenderT" (`self.UniqueRenderT`))
      (`KismetRenderingLibrary.ClearRenderTarget2D` (`self.UniqueRenderT`)))))

(event `Draw`
  (params (Vector2D :type "Vector2D Structure"))
  (bind _drawlocation (`self.DrawLocation`))
  (`MaterialInstanceDynamic.SetVectorParameterValue` _drawlocation "Location" (`KismetMathLibrary.Conv_VectorToLinearColor` (`KismetMathLibrary.Conv_Vector2DToVector` Vector2D)))
  (`KismetRenderingLibrary.DrawMaterialToRenderTarget` (`self.UniqueRenderT`) _drawlocation))

(event `Head Sot`
  (set `self.HitCount` (+ (`self.HitCount`) 1))
  (set `self.TotalScore` (+ (`self.TotalScore`) 100))
  (`KismetSystemLibrary.PrintString` "+100"))

(event `self.ReceiveTick`
  (params (DeltaSeconds :type "Float (single-precision)"))
  (bind (_returnvalue_x _returnvalue_y _returnvalue_z) (`KismetMathLibrary.BreakVector` (`self.K2_GetActorLocation`)))
  ;[1 1 1] Target Movement
  (`|ExecutionSequence`
    (:`then_0`
      (`self.K2_SetActorLocation` (`KismetMathLibrary.MakeVector` _returnvalue_x (`KismetMathLibrary.FClamp` (+ _returnvalue_y (* DeltaSeconds (`self.Move Direction`) (`self.MoveSpeed`))) 840.0 1555.0) _returnvalue_z)))
    (:`then_1`
      (if (>= _returnvalue_y 1555.0)
        (set `self.Move Direction` -1)))
    (:`then_2`
      (if (<= _returnvalue_y 840.0)
        (set `self.Move Direction` 1)))))

(event `Body Shot`
  (set `self.HitCount` (+ (`self.HitCount`) 1))
  (set `self.TotalScore` (+ (`self.TotalScore`) 50))
  (`KismetSystemLibrary.PrintString` "+50"))

(fn `ActivateTarget`
  (params (InMultiplier :type Integer))
  (bind (_returnvalue_x _returnvalue_y _returnvalue_z) (`KismetMathLibrary.BreakVector` (`self.K2_GetActorLocation`)))
  (set `self.HitCount` 0)
  (set `self.TotalScore` 0)
  (set `self.bIsActive` true)
  (`self.K2_SetActorLocation` (`KismetMathLibrary.MakeVector` _returnvalue_x (`KismetMathLibrary.RandomFloatInRange` 840.0 1555.0) _returnvalue_z))
  (if (`KismetMathLibrary.RandomBool`)
    (set `self.Move Direction` 1)
    (else
      (set `self.Move Direction` -1)))
  (set `self.bIsHit` true)
  (bind _output_get (set `self.CalculatedSpeed` (* (`KismetMathLibrary.Conv_IntToDouble` InMultiplier) (`self.BaseTargetSpeed`))))
  (set `self.MoveSpeed` (`KismetMathLibrary.Conv_IntToDouble` _output_get)))

(fn `DeactivateAndResetTarget`
  (bind (_returnvalue_x _returnvalue_y _returnvalue_z) (`KismetMathLibrary.BreakVector` (`self.K2_GetActorLocation`)))
  (set `self.bIsActive` false)
  (set `self.bIsHit` false)
  (set `self.MoveSpeed` 0.0)
  (`self.K2_SetActorLocation` (`KismetMathLibrary.MakeVector` _returnvalue_x 840.0 _returnvalue_z)))

(fn `UserConstructionScript`)