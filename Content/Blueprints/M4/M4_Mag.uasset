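; Grabbable M4 magazine that reloads an M4_Gun when dropped inside its overlap range.
; A collision box, constrained to the mag mesh at BeginPlay, tracks the overlapping gun.
; Grabbing makes the mesh ignore physics bodies.
; On drop, a gun without a magazine reloads, gets flagged as loaded and the mag actor destroys itself; otherwise physics-body blocking is restored.
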(event `self.CollisionBox.OnComponentBeginOverlap`
  (params (OverlappedComponent :type "PrimitiveComponent Object Reference") (OtherActor :type "Actor Object Reference") (OtherComp :type "PrimitiveComponent Object Reference") (OtherBodyIndex :type Integer) (bFromSweep :type Boolean) (SweepResult :type "HitResult Structure (by ref)"))
  (bind _asm4_gun (cast `/Game/Blueprints/M4/M4_Gun` OtherActor))
  (set `self.Gun` _asm4_gun))

(event `self.ReceiveBeginPlay`
  (`PhysicsConstraintComponent.SetConstrainedComponents` (`self.PhysicsConstraint`) (`self.CollisionBox`) "None" (`self.SM_AR4_Mag`) "None"))

(event `self.CollisionBox.OnComponentEndOverlap`
  (params (OverlappedComponent :type "PrimitiveComponent Object Reference") (OtherActor :type "Actor Object Reference") (OtherComp :type "PrimitiveComponent Object Reference") (OtherBodyIndex :type Integer))
  (cast `/Game/Blueprints/M4/M4_Gun` OtherActor)
  (set `self.Gun` null))

(event `self.GrabComponent.FirstOnGrabbed`
  (params (MotionController :type "MotionControllerComponent Object Reference") (MotionControllerAim :type "MotionControllerComponent Object Reference"))
  (`PrimitiveComponent.SetCollisionResponseToChannel` (`self.SM_AR4_Mag`) "ECC_PhysicsBody" "ECR_Ignore"))

(event `self.GrabComponent.FirstOnDropped`
  (`/Engine/EditorBlueprintResources/StandardMacros.IsValid` (`self.Gun`)
    (:`Is Valid`
      (if (`/Game/Blueprints/M4/M4_Gun.IsMagInserted` (`self.Gun`))
        (`PrimitiveComponent.SetCollisionResponseToChannel` (`self.SM_AR4_Mag`) "ECC_PhysicsBody" "ECR_Block" :!label _label)
        (else
          (`/Game/Blueprints/M4/M4_Gun.Reload` (`self.Gun`))
          (set `/Game/Blueprints/M4/M4_Gun.IsMagInserted` true (`self.Gun`))
          (`self.K2_DestroyActor`))))
    (:`Is Not Valid`
      (goto _label))))

(fn `UserConstructionScript`)