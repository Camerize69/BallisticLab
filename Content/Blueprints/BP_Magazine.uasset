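; BP_Magazine is a weapon magazine that tracks its round count and provides sounds for going in and out.
; RemoveRound decrements Rounds, then calls HasRound, which shows or hides the Round component and sets IsEmpty when the count is zero.
; The construction script also runs HasRound to match the starting count.
; PlayInSound and PlayOutSound play their sounds at the magazine mesh's location.
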(fn `HasRound`
  (bind _round (`self.Round`))
  (if (== (`self.Rounds`) 0)
    (`SceneComponent.SetVisibility` _round false false)
    (set `self.IsEmpty` true)
    (else
      (`SceneComponent.SetVisibility` _round true false)
      (set `self.IsEmpty` false)))
  (return))

(fn `PlayInSound`
  (`GameplayStatics.PlaySoundAtLocation` (`self.MagInSound`) (`SceneComponent.K2_GetComponentLocation` (`self.MagazineMesh`)) (struct) 1.0 1.0 0.0 null null null null))

(fn `PlayOutSound`
  (`GameplayStatics.PlaySoundAtLocation` (`self.MagOutSound`) (`SceneComponent.K2_GetComponentLocation` (`self.MagazineMesh`)) (struct) 1.0 1.0 0.0 null null null null))

(fn `RemoveRound`
  (`/Engine/EditorBlueprintResources/StandardMacros.DecrementInt` (`self.Rounds`)
    (:`  `
      (`self.HasRound`))))

(fn `UserConstructionScript`
  (`self.HasRound`))