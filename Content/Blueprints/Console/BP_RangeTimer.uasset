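; BP_RangeTimer is a countdown timer for shooting range sessions.
; StartTimer stores the truncated duration and starts a looping one-second timer that decrements the remaining time.
; At zero, StopAndResetTimer clears the timer, deactivates and resets all Target_BP actors in the level, and clears the running flag.
; BeginPlay caches a BP_ShootingRangeConsole reference, though these graphs never use it.
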(event `self.ReceiveBeginPlay`
  (bind _returnvalue (`GameplayStatics.GetActorOfClass` "/Game/Blueprints/Console/BP_ShootingRangeConsole.BP_ShootingRangeConsole_C"))
  (set `self.ConsoleRef` _returnvalue))

(event `StartTimer`
  (params (InDuration :type "Float (double-precision)"))
  (bind _returnvalue (`KismetMathLibrary.FTrunc` InDuration))
  (set `self.bIsRunning` true)
  (set `self.SessionDuration` _returnvalue)
  (set `self.RemainingTime` _returnvalue)
  (bind _returnvalue_2 (`KismetSystemLibrary.K2_SetTimerDelegate` (delegate `TickTimer`) 1.0 true))
  (set `self.TimerHandle` _returnvalue_2))

(event `TickTimer`
  (bind _remainingtime (`self.RemainingTime`))
  (set `self.RemainingTime` (- _remainingtime 1))
  (if (<= _remainingtime 0)
    (`self.StopAndResetTimer`)))

(event `StopAndResetTimer`
  (`KismetSystemLibrary.K2_ClearAndInvalidateTimerHandle` (`self.TimerHandle`))
  (bind _outactors (`GameplayStatics.GetAllActorsOfClass` "/Game/Blueprints/Target_BP.Target_BP_C"))
  (`/Game/Blueprints/Target_BP.DeactivateAndResetTarget` _outactors)
  (set `self.bIsRunning` false))

(fn `UserConstructionScript`)