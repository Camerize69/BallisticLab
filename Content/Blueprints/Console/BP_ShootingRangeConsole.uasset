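; Shooting range console that lets the player set target speed and start or stop a timed round.
; Overlapping the Up and Down boxes steps a clamped speed multiplier after a short delay and updates the WBP_SpeedDisplay widget.
; The Start box toggles the round: starting activates every Target_BP at that speed and runs the BP_RangeTimer found at BeginPlay.
; Stopping only resets the timer and active flag, without signalling the targets.
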(event `self.ReceiveBeginPlay`
  (bind _returnvalue (`GameplayStatics.GetActorOfClass` "/Game/Blueprints/Console/BP_RangeTimer.BP_RangeTimer_C"))
  (set `self.RangeTimerRef` _returnvalue)
  (bind _aswbp_speed_display (cast `/Game/Blueprints/Console/WBP_SpeedDisplay` (`WidgetComponent.GetUserWidgetObject` (`self.Widget_Display`))))
  (`/Game/Blueprints/Console/WBP_SpeedDisplay.UpdateSpeedDisplay` _aswbp_speed_display (`self.SpeedMultiplier`)))

(event `self.Box_Up.OnComponentBeginOverlap`
  (params (OverlappedComponent :type "PrimitiveComponent Object Reference") (OtherActor :type "Actor Object Reference") (OtherComp :type "PrimitiveComponent Object Reference") (OtherBodyIndex :type Integer) (bFromSweep :type Boolean) (SweepResult :type "HitResult Structure (by ref)"))
  (`KismetSystemLibrary.Delay` 0.2)
  (bind _output_get (set `self.SpeedMultiplier` (`KismetMathLibrary.Clamp` (+ (`self.SpeedMultiplier`) 1) 1 5)))
  (bind _aswbp_speed_display (cast `/Game/Blueprints/Console/WBP_SpeedDisplay` (`WidgetComponent.GetUserWidgetObject` (`self.Widget_Display`))))
  (`/Game/Blueprints/Console/WBP_SpeedDisplay.UpdateSpeedDisplay` _aswbp_speed_display _output_get))

(event `self.Box_Down.OnComponentBeginOverlap`
  (params (OverlappedComponent :type "PrimitiveComponent Object Reference") (OtherActor :type "Actor Object Reference") (OtherComp :type "PrimitiveComponent Object Reference") (OtherBodyIndex :type Integer) (bFromSweep :type Boolean) (SweepResult :type "HitResult Structure (by ref)"))
  (`KismetSystemLibrary.Delay` 0.2)
  (bind _output_get (set `self.SpeedMultiplier` (`KismetMathLibrary.Clamp` (- (`self.SpeedMultiplier`) 1) 1 5)))
  (bind _aswbp_speed_display (cast `/Game/Blueprints/Console/WBP_SpeedDisplay` (`WidgetComponent.GetUserWidgetObject` (`self.Widget_Display`))))
  (`/Game/Blueprints/Console/WBP_SpeedDisplay.UpdateSpeedDisplay` _aswbp_speed_display _output_get))

(event `self.Box_Start.OnComponentBeginOverlap`
  (params (OverlappedComponent :type "PrimitiveComponent Object Reference") (OtherActor :type "Actor Object Reference") (OtherComp :type "PrimitiveComponent Object Reference") (OtherBodyIndex :type Integer) (bFromSweep :type Boolean) (SweepResult :type "HitResult Structure (by ref)"))
  (if (not (`self.bIsGameActive`))
    (set `self.bIsGameActive` true)
    (bind _outactors (`GameplayStatics.GetAllActorsOfClass` "/Game/Blueprints/Target_BP.Target_BP_C"))
    (`/Game/Blueprints/Target_BP.ActivateTarget` _outactors (`self.SpeedMultiplier`))
    (`/Game/Blueprints/Console/BP_RangeTimer.StartTimer` (`self.RangeTimerRef`) 30.0)
    (else
      (`/Game/Blueprints/Console/BP_RangeTimer.StopAndResetTimer` (`self.RangeTimerRef`))
      (set `self.bIsGameActive` false))))

(fn `UserConstructionScript`)