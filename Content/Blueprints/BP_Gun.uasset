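; VR gun actor with grab-driven input, a hand-pulled charging handle and physical magazines.
; Grabbing adds per-hand mapping contexts; the analog trigger animates finger and trigger, firing a muzzle line trace with decal and sounds, in semi-auto only.
; Timer-driven slide movement tracks chambered rounds, ejection and dry-fire state, with sounds and haptics.
; Held magazines of matching type snap into the socket on overlap; inputs drop them or cycle fire modes.
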(event `self.ReceiveBeginPlay`
  (if (not (`self.HasFiringMode`))
    (`KismetSystemLibrary.PrintString` "NO FIRING MODE ADDED TO THE GUN" true true (struct :`R` 1.0 :`G` 0.019076 :`A` 1.0))))

(event `self.MainGrabComponent.OnGrabbed`
  (params (MotionController :type "MotionControllerComponent Object Reference"))
  ;[0.03434 0.03434 0.03434] Main Grab
  (`self.Motion Controller`
    (:`then`
      (`EnhancedInputSubsystemInterface.RemoveMappingContext` (pcsubsystem `EnhancedInputLocalPlayerSubsystem` (`GameplayStatics.GetPlayerController` 0)) (select `bool` (`|EnumEquality` (`/Game/Blueprints/GrabComponent.GetHeldByHand` (`self.MainGrabComponent`)) "Right") :`false` "/Game/VRTemplate/Input/IMC_Weapon_Right.IMC_Weapon_Right" :`true` "/Game/VRTemplate/Input/IMC_Weapon_Left.IMC_Weapon_Left" :!type "InputMappingContext Object Reference") (struct))
      (set `self.Motion Controller` null))
    (:`else`
      _))
  (set `self.Motion Controller` MotionController)
  (bind _holdinghandanim (`self.GetHoldingHandAnim`))
  (set `self.Holding Hand Anim` _holdinghandanim)
  (`self.EnableInput` (`GameplayStatics.GetPlayerController` 0))
  (`EnhancedInputSubsystemInterface.AddMappingContext` (pcsubsystem `EnhancedInputLocalPlayerSubsystem` (`GameplayStatics.GetPlayerController` 0)) (select `bool` (`|EnumEquality` (`/Game/Blueprints/GrabComponent.GetHeldByHand` (`self.MainGrabComponent`)) "Left") :`false` "/Game/VRTemplate/Input/IMC_Weapon_Right.IMC_Weapon_Right" :`true` "/Game/VRTemplate/Input/IMC_Weapon_Left.IMC_Weapon_Left" :!type "InputMappingContext Object Reference") 1 (struct)))

(event `self.MainGrabComponent.OnDropped`
  ;[0.03434 0.03434 0.03434] Main Grab
  (`self.DisableInput` (`GameplayStatics.GetPlayerController` 0))
  (`EnhancedInputSubsystemInterface.RemoveMappingContext` (pcsubsystem `EnhancedInputLocalPlayerSubsystem` (`GameplayStatics.GetPlayerController` 0)) (select `bool` (`|EnumEquality` (`/Game/Blueprints/GrabComponent.GetHeldByHand` (`self.MainGrabComponent`)) "Left") :`false` "/Game/VRTemplate/Input/IMC_Weapon_Right.IMC_Weapon_Right" :`true` "/Game/VRTemplate/Input/IMC_Weapon_Left.IMC_Weapon_Left" :!type "InputMappingContext Object Reference") (struct)))

(event `EnhancedInput|/Game/VRTemplate/Input/Actions/IA_Shoot_Left`
  (params (ActionValue :type "Float (double-precision)") (ElapsedSeconds :type "Float (double-precision)") (TriggeredSeconds :type "Float (double-precision)") (InputAction :type "InputAction Object Reference" :default "/Game/VRTemplate/Input/Actions/IA_Shoot_Left.IA_Shoot_Left"))
  (:`Triggered`
    (switch `/Game/Blueprints/Enums/FiringMode` (`self.CurrentFiringMode`)
      (:`NewEnumerator1`
        _)
      (:`NewEnumerator2`
        _)
      (:`NewEnumerator3`
        _))
    (bind _output_get (set `self.ActionValueLeft` ActionValue))
    (set `/Game/Hands/QK_CustomHand_ABP.TriggerPressValue` _output_get (`self.Holding Hand Anim`))
    (`SceneComponent.K2_SetRelativeRotation` (`self.Trigger`) (`KismetMathLibrary.RLerp` (struct) (`self.TriggerMaxRotation`) (`self.ActionValueLeft`)) false false)
    (if (> (`self.ActionValueLeft`) (`self.FireTHreshold`))
      (if (`self.HasFiringMode`) :!label _label
        (switch `/Game/Blueprints/Enums/FiringMode` (`self.CurrentFiringMode`)
          (:`NewEnumerator1`
            (`/Engine/EditorBlueprintResources/StandardMacros.DoOnce` false :!label _label_2
              (:`Completed`
                (`self.SingleShot`))))))
      (else
        (goto _label_2 :!via `Reset`))))
  (:`Canceled`
    (switch `/Game/Blueprints/Enums/FiringMode` (`self.CurrentFiringMode`) :!label _label_3
      (:`NewEnumerator1`
        _)
      (:`NewEnumerator2`
        _)
      (:`NewEnumerator3`
        _))
    (set `self.ActionValueLeft` 0.0)
    (set `/Game/Hands/QK_CustomHand_ABP.TriggerPressValue` 0.0 (`self.Holding Hand Anim`))
    (goto _label_2 :!via `Reset`))
  (:`Completed`
    (goto _label_3)))

(event `EnhancedInput|/Game/VRTemplate/Input/Actions/IA_Shoot_Right`
  (params (ActionValue :type "Float (double-precision)") (ElapsedSeconds :type "Float (double-precision)") (TriggeredSeconds :type "Float (double-precision)") (InputAction :type "InputAction Object Reference" :default "/Game/VRTemplate/Input/Actions/IA_Shoot_Right.IA_Shoot_Right"))
  (:`Triggered`
    (switch `/Game/Blueprints/Enums/FiringMode` (`self.CurrentFiringMode`)
      (:`NewEnumerator1`
        _)
      (:`NewEnumerator2`
        _)
      (:`NewEnumerator3`
        _))
    (bind _output_get (set `self.ActionValueRight` ActionValue))
    (set `/Game/Hands/QK_CustomHand_ABP.TriggerPressValue` _output_get (`self.Holding Hand Anim`))
    (`SceneComponent.K2_SetRelativeRotation` (`self.Trigger`) (`KismetMathLibrary.RLerp` (struct) (`self.TriggerMaxRotation`) (`self.ActionValueRight`)) false false)
    (if (> (`self.ActionValueRight`) (`self.FireTHreshold`))
      (goto _label)
      (else
        (goto _label_2 :!via `Reset`))))
  (:`Canceled`
    (switch `/Game/Blueprints/Enums/FiringMode` (`self.CurrentFiringMode`) :!label _label_4
      (:`NewEnumerator1`
        _)
      (:`NewEnumerator2`
        _)
      (:`NewEnumerator3`
        _))
    (set `self.ActionValueRight` 0.0)
    (set `/Game/Hands/QK_CustomHand_ABP.TriggerPressValue` 0.0 (`self.Holding Hand Anim`))
    (goto _label_2 :!via `Reset`))
  (:`Completed`
    (goto _label_4)))

(event `self.CurlGrabComponent.OnGrabbed`
  (params (MotionController :type "MotionControllerComponent Object Reference"))
  (`self.AttachHandToSlide` MotionController)
  (`GameplayStatics.PlaySoundAtLocation` (`self.SlideGrabbedSound`) (`SceneComponent.K2_GetComponentLocation` (`self.SlideGrabCollision`)) (struct) 1.0 1.0 0.0 null null null null)
  (set `self.Initial Grab Offset` (`self.GetGrabbedOffestBwtweenMC&Slide`))
  (set `self.SliderReleased` false)
  (`KismetSystemLibrary.K2_SetTimerDelegate` (delegate `Interpolate Slide Movement`) 0.01 true))

(event `Interpolate Slide Movement`
  (bind _round (`self.Round`))
  (bind _returnvalue (`self.ClampSlideMovement` (`self.ChargingHandleMaxDistance`)))
  (set `self.CurrentSlideOffset` _returnvalue)
  (if (and (== _returnvalue (`self.ChargingHandleMaxDistance`)) (not (`self.ReachedLockPosition`)))
    (set `self.ReachedLockPosition` true)
    (`GameplayStatics.PlaySoundAtLocation` (`self.CockedSound`) (`SceneComponent.K2_GetComponentLocation` (`self.SlideGrabCollision`)) (struct) 1.0 1.0 0.0 null null null null)
    (bind _magazine (`self.Magazine`)
      (:`then`
        (if (`/Game/Blueprints/BP_Magazine.IsEmpty` _magazine)
          (set `self.DryFire` true :!label _label)
          (set `self.BulletIsReadyToBeTakenFromMag` false)
          (else
            (set `self.DryFire` false)
            (set `self.BulletIsReadyToBeTakenFromMag` true))))
      (:`else`
        (goto _label)))
    (if (`self.ChamberHasBullet`)
      (`self.InitiateBulletThrowAndSetRoundMesVisible`))
    (`self.PlayHapticEffect` 0.8)
    (elif (`self.ReachedLockPosition`)
      (if (<= (`self.CurrentSlideOffset`) (- (`self.ChargingHandleMaxDistance`) (`self.DistanceToTrabelBackFromLockToGetBullet`)))
        (bind _magazine_2 (`self.Magazine`)
          (:`then`
            (if (`/Game/Blueprints/BP_Magazine.IsEmpty` _magazine_2)
              (`SceneComponent.SetVisibility` _round false false)
              (set `self.ChamberHasBullet` false)
              (else
                (`SceneComponent.SetVisibility` _round true false)
                (`/Game/Blueprints/BP_Magazine.RemoveRound` _magazine_2)
                (set `self.ChamberHasBullet` true)))
            (set `self.ReachedLockPosition` false))
          (:`else`
            _)))))
  (`SceneComponent.K2_SetRelativeLocation` (`self.Handle`) (`KismetMathLibrary.MakeVector` (`self.CurrentSlideOffset`)) false false))

(event `self.CurlGrabComponent.OnDropped`
  (`self.DetachHandFromSlide`)
  (set `self.SlideGrabMotionController` null)
  (set `self.SlideMotionControllerHandMesh` null)
  (`KismetSystemLibrary.K2_PauseTimer` null "Interpolate Slide Movement")
  (if (not (<= (`self.CurrentSlideOffset`) (`self.OffsetToPlayReleasedSound`)))
    (`GameplayStatics.PlaySoundAtLocation` (`self.SlideReleasedSound`) (`SceneComponent.K2_GetComponentLocation` (`self.Slide`)) (struct) 1.0 1.0 0.0 null null null null)
    (`self.PlayHapticEffectOnOppositeHand` 1.0))
  (set `self.SliderReleased` true)
  (`KismetSystemLibrary.K2_SetTimerDelegate` (delegate `Return Slide Back`) 0.01 true))

(event `Return Slide Back`
  (bind _hasreachedorigin (`self.InterpolateHandleToInitialPositionAndContinueOnceDone`))
  (if _hasreachedorigin
    (`SceneComponent.K2_SetRelativeLocation` (`self.Handle`) (0.0 0.0 0.0) false false)
    (`KismetSystemLibrary.K2_PauseTimer` null "Return Slide Back")
    (set `self.CurrentSlideOffset` 0.0)
    (if (`self.ReachedLockPosition`)
      (bind _magazine (`self.Magazine`)
        (:`then`
          (if (`self.BulletIsReadyToBeTakenFromMag`)
            (if (`/Game/Blueprints/BP_Magazine.IsEmpty` _magazine)
              (if (not (`self.ChamberHasBullet`))
                (set `self.DryFire` true :!label _label_2)
                (`SceneComponent.SetVisibility` (`self.Round`) false false)
                (set `self.ChamberHasBullet` false)
                (set `self.ReachedLockPosition` false :!label _label_3))
              (else
                (`/Game/Blueprints/BP_Magazine.RemoveRound` (`self.Magazine`))
                (`SceneComponent.SetVisibility` (`self.Round`) true false)
                (set `self.ChamberHasBullet` true)
                (goto _label_3)))
            (else
              (set `self.ReachedLockPosition` false :!label _label_4)
              (goto _label_2))))
        (:`else`
          (goto _label_4))))))

(event `self.MagazineCollision.OnComponentBeginOverlap`
  (params (OverlappedComponent :type "PrimitiveComponent Object Reference") (OtherActor :type "Actor Object Reference") (OtherComp :type "PrimitiveComponent Object Reference") (OtherBodyIndex :type Integer) (bFromSweep :type Boolean) (SweepResult :type "HitResult Structure (by ref)"))
  (bind _magazine (`self.Magazine`))
  (bind _curlgrabcomponent (`/Game/Blueprints/BP_Magazine.CurlGrabComponent` _magazine))
  (`self.Magazine`
    (:`then`)
    (:`else`
      (bind _asbp_magazine (cast `/Game/Blueprints/BP_Magazine` OtherActor))
      (if (`|EnumEquality` (`/Game/Blueprints/BP_Magazine.MagazineType` _asbp_magazine) (`self.GunType`))
        (if (`/Game/Blueprints/CurlGrabComponent.bIsHeld` (`/Game/Blueprints/BP_Magazine.CurlGrabComponent` _asbp_magazine))
          (bind _output_get (set `self.Magazine` _asbp_magazine))
          (`PrimitiveComponent.SetSimulatePhysics` (`/Game/Blueprints/BP_Magazine.MagazineMesh` _output_get) false)
          (set `/Game/Blueprints/CurlGrabComponent.bSimulateOnDrop` false (`/Game/Blueprints/BP_Magazine.CurlGrabComponent` _output_get))
          (`/Game/Blueprints/BP_Magazine.PlayInSound` _magazine)
          (`/Game/Blueprints/CurlGrabComponent.TryRelease` _curlgrabcomponent)
          (add `/Game/Blueprints/CurlGrabComponent.OnGrabbed` _curlgrabcomponent (delegate `SimulateMagazinePhysicsOnDropped`))
          (`KismetSystemLibrary.K2_SetTimerDelegate` (delegate `Smooth Attachment`) 0.001 true))))))

(event `SimulateMagazinePhysicsOnDropped`
  (params (MotionController :type "MotionControllerComponent Object Reference"))
  (bind _curlgrabcomponent (`/Game/Blueprints/BP_Magazine.CurlGrabComponent` (`self.Magazine`)))
  (set `/Game/Blueprints/CurlGrabComponent.bSimulateOnDrop` true _curlgrabcomponent)
  (remove `/Game/Blueprints/CurlGrabComponent.OnGrabbed` _curlgrabcomponent (delegate `SimulateMagazinePhysicsOnDropped`))
  (set `self.Magazine` null))

(event `Smooth Attachment`
  (bind _returnvalue (`self.SmoothMagazineAttachmentAndContinueOnceDone`))
  (if _returnvalue
    (`self.K2_AttachToComponent` (`self.Magazine`) (`self.GunMesh`) "Magazine" "SnapToTarget" "SnapToTarget" "SnapToTarget" true)
    (`KismetSystemLibrary.K2_PauseTimer` null "Smooth Attachment")))

(event `EnhancedInput|/Game/VRTemplate/Input/Actions/IA_SwitchFiringMode_Left`
  (params (ActionValue :type Boolean) (ElapsedSeconds :type "Float (double-precision)") (TriggeredSeconds :type "Float (double-precision)") (InputAction :type "InputAction Object Reference" :default "/Game/VRTemplate/Input/Actions/IA_SwitchFiringMode_Left.IA_SwitchFiringMode_Left"))
  (:`Completed`
    (`self.SwitchGunMode` :!label _label)))

(event `EnhancedInput|/Game/VRTemplate/Input/Actions/IA_SwitchFiringMode_Right`
  (params (ActionValue :type Boolean) (ElapsedSeconds :type "Float (double-precision)") (TriggeredSeconds :type "Float (double-precision)") (InputAction :type "InputAction Object Reference" :default "/Game/VRTemplate/Input/Actions/IA_SwitchFiringMode_Right.IA_SwitchFiringMode_Right"))
  (:`Completed`
    (goto _label)))

(event `EnhancedInput|/Game/VRTemplate/Input/Actions/IA_DropMag_Left`
  (params (ActionValue :type Boolean) (ElapsedSeconds :type "Float (double-precision)") (TriggeredSeconds :type "Float (double-precision)") (InputAction :type "InputAction Object Reference" :default "/Game/VRTemplate/Input/Actions/IA_DropMag_Left.IA_DropMag_Left"))
  (bind _curlgrabcomponent (`/Game/Blueprints/BP_Magazine.CurlGrabComponent` (`self.Magazine`)))
  (:`Completed`
    (bind _magazine (`self.Magazine` :!label _label_2)
      (:`then`
        (`/Game/Blueprints/BP_Magazine.PlayOutSound` _magazine)
        (bind _magazinemesh (`/Game/Blueprints/BP_Magazine.MagazineMesh` _magazine))
        (`SceneComponent.K2_DetachFromComponent` _magazinemesh "KeepWorld" "KeepWorld" "KeepWorld" true)
        (`PrimitiveComponent.SetSimulatePhysics` _magazinemesh true)
        (clear `/Game/Blueprints/CurlGrabComponent.OnGrabbed` _curlgrabcomponent)
        (set `/Game/Blueprints/CurlGrabComponent.bSimulateOnDrop` true _curlgrabcomponent)
        (set `self.Magazine` null))
      (:`else`))))

(event `EnhancedInput|/Game/VRTemplate/Input/Actions/IA_DropMag_Right`
  (params (ActionValue :type Boolean) (ElapsedSeconds :type "Float (double-precision)") (TriggeredSeconds :type "Float (double-precision)") (InputAction :type "InputAction Object Reference" :default "/Game/VRTemplate/Input/Actions/IA_DropMag_Right.IA_DropMag_Right"))
  (:`Completed`
    (goto _label_2)))

(fn `AttachHandToSlide`
  (params (MotionContoller :type "MotionControllerComponent Object Reference"))
  (bind _curlgrabcomponent (`self.CurlGrabComponent`))
  (set `self.SlideGrabMotionController` MotionContoller)
  (if (`|EnumEquality` (`/Game/Blueprints/CurlGrabComponent.GetHeldByHand` _curlgrabcomponent) "Right")
    (bind _output_get (set `self.SlideMotionControllerHandMesh` (`/Game/Blueprints/CurlGrabComponent.Hand Right` _curlgrabcomponent)))
    (`SceneComponent.K2_AttachToComponent` _output_get (`self.SlideHand_R`) "None" "SnapToTarget" "SnapToTarget" "KeepRelative" true)
    (else
      (bind _output_get_2 (set `self.SlideMotionControllerHandMesh` (`/Game/Blueprints/CurlGrabComponent.Hand Left` _curlgrabcomponent)))
      (`SceneComponent.K2_AttachToComponent` _output_get_2 (`self.SlideHand_L`) "None" "SnapToTarget" "SnapToTarget" "KeepRelative" true)))
  (return))

(fn `BulletDefaultHitDecal`
  (params (`Hit Component` :type "PrimitiveComponent Object Reference") (`Hit Location` :type "Vector Structure") (Normal :type "Vector Structure"))
  (bind _returnvalue (`GameplayStatics.SpawnDecalAttached` "/Game/Materials/M_Bullet_decal.M_Bullet_decal" (2.0 2.0 2.0) `Hit Component` "None" `Hit Location` (`KismetMathLibrary.Conv_VectorToRotator` Normal) "KeepRelativeOffset" 10.0))
  (`/Engine/EditorBlueprintResources/StandardMacros.IsValid` _returnvalue))

(fn `ClampSlideMovement`
  (params (Min :type "Float (double-precision)"))
  (returns (ReturnValue :type "Float (double-precision)"))
  (bind _relativelocation_x (`KismetMathLibrary.BreakVector` (`SceneComponent.RelativeLocation` (`self.Handle`))))
  (bind _returnvalue_x (`KismetMathLibrary.BreakVector` (`KismetMathLibrary.InverseTransformLocation` (`SceneComponent.K2_GetComponentToWorld` (`self.Handle`)) (- (`SceneComponent.K2_GetComponentLocation` (`/Game/Blueprints/CurlGrabComponent.MotionControllerRef` (`self.CurlGrabComponent`))) (`self.Initial Grab Offset`)))))
  (bind _returnvalue (+ _returnvalue_x _relativelocation_x))
  (return (select `bool` (< (`self.ChargingHandleMaxDistance`) 0.0) :`false` (`KismetMathLibrary.FClamp` _returnvalue 0.0 Min) :`true` (`KismetMathLibrary.FClamp` Min _returnvalue 0.0))))

(fn `DetachHandFromSlide`
  (bind _slidemotioncontrollerhandmesh (`self.SlideMotionControllerHandMesh`))
  (`SceneComponent.K2_AttachToComponent` (`self.SlideMotionControllerHandMesh`) (`self.SlideGrabMotionController`) "None" "SnapToTarget" "SnapToTarget" "SnapToTarget" true)
  (if (`|EnumEquality` (`/Game/Blueprints/CurlGrabComponent.GetHeldByHand` (`self.CurlGrabComponent`)) "Right")
    (`SceneComponent.K2_SetRelativeRotation` _slidemotioncontrollerhandmesh (struct :`Pitch` -53.0 :`Yaw` -13.5 :`Roll` 106.8) false false)
    (else
      (`SceneComponent.K2_SetRelativeRotation` _slidemotioncontrollerhandmesh (struct :`Pitch` -53.7 :`Yaw` 32.64 :`Roll` 265.9) false false)
      (`SceneComponent.SetRelativeScale3D` _slidemotioncontrollerhandmesh (* (`SceneComponent.RelativeScale3D` _slidemotioncontrollerhandmesh) (1.0 -1.0 1.0)))))
  (`SceneComponent.K2_SetRelativeLocation` _slidemotioncontrollerhandmesh (-2.98126 -3.5 4.561753) false false)
  (return))

(fn `GetGrabbedOffestBwtweenMC&Slide`
  (returns (InitialOffset :type "Vector Structure"))
  (return (- (`SceneComponent.K2_GetComponentLocation` (`/Game/Blueprints/CurlGrabComponent.MotionControllerRef` (`self.CurlGrabComponent`))) (`SceneComponent.K2_GetComponentLocation` (`self.Handle`)))))

(fn `GetHoldingHandAnim`
  (returns (HoldingHandAnim :type "/Game/Hands/QK_CustomHand_ABP Object Reference"))
  (bind _maingrabcomponent (`self.MainGrabComponent`))
  (if (`|EnumEquality` (`/Game/Blueprints/GrabComponent.GetHeldByHand` _maingrabcomponent) "Left")
    (return (`/Game/Blueprints/GrabComponent.LeftHandAnim` _maingrabcomponent))
    (else
      (return (`/Game/Blueprints/GrabComponent.RightHandAnim` _maingrabcomponent)))))

(fn `Gun Location & Direction`
  (params (Distance :type "Float (double-precision)"))
  (returns (Location :type "Vector Structure") (Direction :type "Vector Structure"))
  (bind (_returnvalue_location _returnvalue_rotation) (`KismetMathLibrary.BreakTransform` (`SceneComponent.K2_GetComponentToWorld` (`self.Muzzle`))))
  (return _returnvalue_location (+ _returnvalue_location (* (`KismetMathLibrary.GetForwardVector` _returnvalue_rotation) Distance))))

(fn `HasFiringMode`
  (returns (HasAtLeastOneFiringMode :type Boolean))
  (return (> (`KismetArrayLibrary.Array_Length` (`self.FiringModes`)) 0)))

(fn `ImpactDecals`
  (params (Hit :type "HitResult Structure"))
  (bind (_bblockinghit _binitialoverlap _time _distance _location _impactpoint _normal _impactnormal _physmat _hitactor _hitcomponent) (`GameplayStatics.BreakHitResult` Hit))
  (`self.BulletDefaultHitDecal` _hitcomponent _impactpoint _normal)
  (return))

(fn `ImpactSoundsAndParticles`
  (params (Hit :type "HitResult Structure"))
  (bind (_bblockinghit _binitialoverlap _time _distance _location _impactpoint) (`GameplayStatics.BreakHitResult` Hit))
  (if _bblockinghit
    (`GameplayStatics.SpawnSoundAtLocation` "/Game/Sounds/Cue_BulletImpactConcrete.Cue_BulletImpactConcrete" _impactpoint (struct) 2.0 1.0 0.0 "/Game/Sounds/BulletImpactAttenuation.BulletImpactAttenuation" null)))

(fn `InitiateBulletThrowAndSetRoundMesVisible`
  (bind (_returnvalue_location _returnvalue_rotation _returnvalue_scale) (`KismetMathLibrary.BreakTransform` (`SceneComponent.K2_GetComponentToWorld` (`self.Round`))))
  (`NiagaraFunctionLibrary.SpawnSystemAtLocation` (`self.SlideRoundEjection`) _returnvalue_location _returnvalue_rotation _returnvalue_scale)
  (`SceneComponent.SetVisibility` (`self.Round`) false false)
  (return))

(fn `InterpolateHandleToInitialPositionAndContinueOnceDone`
  (returns (HasReachedOrigin :type Boolean))
  (bind _handle (`self.Handle`))
  (bind _relativelocation_x (`KismetMathLibrary.BreakVector` (`SceneComponent.RelativeLocation` _handle)))
  (bind _returnvalue (`KismetMathLibrary.FInterpTo` _relativelocation_x 0.0 (* (`GameplayStatics.GetWorldDeltaSeconds`) (`self.SldierSnapToOriginSpeedMultiplier`)) 0.4))
  (`SceneComponent.K2_SetRelativeLocation` _handle (`KismetMathLibrary.MakeVector` _returnvalue) false false)
  (return (`KismetMathLibrary.NearlyEqual_FloatFloat` _returnvalue 0.0 0.001)))

(fn `Line Trace From Barrel`
  (params (Start :type "Vector Structure") (End :type "Vector Structure"))
  (returns (OutHit :type "HitResult Structure"))
  (bind _outhit (`KismetSystemLibrary.LineTraceSingle` :`Start` Start :`End` End :`TraceChannel` "TraceTypeQuery1" :`DrawDebugType` "ForDuration" :`DrawTime` 3.0))
  (return _outhit))

(fn `Line Trace, Impact Decals, Randomizing Recoil & Sound`
  (bind (_location _direction) (`self.Gun Location & Direction` -2000.0))
  (`GameplayStatics.PlaySoundAtLocation` (`self.ShotSound`) (`SceneComponent.K2_GetComponentLocation` (`self.Muzzle`)) (struct) 1.0 1.0 0.0 null null null null)
  (bind _outhit (`self.Line Trace From Barrel` _location _direction))
  (`self.ImpactDecals` _outhit)
  (`self.RandomizedRecoil`)
  (`self.ImpactSoundsAndParticles` _outhit))

(fn `PlayHapticEffect`
  (params (Scale :type "Float (double-precision)"))
  (`PlayerController.PlayHapticEffect` (`GameplayStatics.GetPlayerController` 0) (`self.HapticEffect`) (`/Game/Blueprints/CurlGrabComponent.GetHeldByHand` (`self.CurlGrabComponent`)) Scale false)
  (return))

(fn `PlayHapticEffectOnOppositeHand`
  (params (Scale :type "Float (double-precision)"))
  (bind _returnvalue (`GameplayStatics.GetPlayerController` 0))
  (bind _hapticeffect (`self.HapticEffect`))
  (if (`|EnumEquality` (`/Game/Blueprints/CurlGrabComponent.GetHeldByHand` (`self.CurlGrabComponent`)) "Left")
    (`PlayerController.PlayHapticEffect` _returnvalue _hapticeffect "Right" Scale false)
    (else
      (`PlayerController.PlayHapticEffect` _returnvalue _hapticeffect "Left" Scale false)))
  (return))

(fn `RandomizedRecoil`
  (set `self.RandomRecoilY` (`KismetMathLibrary.RandomFloatInRange` -0.65 0.65))
  (set `self.RandomRecoilZ` (`KismetMathLibrary.RandomFloatInRange` 0.0 0.75)))

(fn `SingleShot`
  (`self.Magazine`
    (:`then`
      (if (`self.ChamberHasBullet`)
        (if (`/Game/Blueprints/BP_Magazine.IsEmpty` (`self.Magazine`))
          (if (`self.SliderReleased`) :!label _label
            (set `self.ChamberHasBullet` false)
            (`SceneComponent.SetVisibility` (`self.Round`) false false)
            (`self.Line Trace, Impact Decals, Randomizing Recoil & Sound`)
            (`self.StoreGunLocation&Rotation`)
            (else
              (if (`self.DryFire`) :!label _label_2
                (`GameplayStatics.PlaySoundAtLocation` (`self.DryFireSound`) (`SceneComponent.K2_GetComponentLocation` (`self.Trigger`)) (struct) 1.0 1.0 0.0 null null null null)
                (set `self.DryFire` false)
                (else
                  (`GameplayStatics.PlaySoundAtLocation` (`self.EmptyTriggerSound`) (`SceneComponent.K2_GetComponentLocation` (`self.Trigger`)) (struct) 1.0 1.0 0.0 null null null null)))))
          (elif (`self.SliderReleased`)
            (`/Game/Blueprints/BP_Magazine.RemoveRound` (`self.Magazine`))
            (`self.Line Trace, Impact Decals, Randomizing Recoil & Sound`)
            (`self.StoreGunLocation&Rotation`)
            (else
              (goto _label_2))))
        (else
          (goto _label_2))))
    (:`else`
      (if (`self.ChamberHasBullet`)
        (goto _label)
        (else
          (goto _label_2))))))

(fn `SmoothMagazineAttachmentAndContinueOnceDone`
  (returns (ReturnValue :type Boolean))
  (bind _magazine (`self.Magazine`))
  (bind _returnvalue (`SceneComponent.GetSocketLocation` (`self.GunMesh`) "Magazine"))
  (bind _returnvalue_2 (`KismetMathLibrary.VInterpTo` (`SceneComponent.K2_GetComponentLocation` (`/Game/Blueprints/BP_Magazine.MagazineMesh` _magazine)) _returnvalue (* (`GameplayStatics.GetWorldDeltaSeconds`) (`self.MagazineSnapSpeedMultiplier`))))
  (`SceneComponent.K2_SetRelativeLocation` (`Actor.RootComponent` _magazine) _returnvalue_2 false false)
  (return (== _returnvalue _returnvalue_2 :`ErrorTolerance` 0.01)))

(fn `StoreGunLocation&Rotation`
  (bind (_returnvalue_location _returnvalue_rotation) (`KismetMathLibrary.BreakTransform` (`SceneComponent.GetRelativeTransform` (`self.GunMesh`))))
  (set `self.Relative Location` _returnvalue_location)
  (set `self.Relative Rotation` _returnvalue_rotation)
  (return))

(fn `SwitchGunMode`
  (if (`self.HasFiringMode`)
    (if (== (`self.CurrentFiringModeIndex`) (- (`KismetArrayLibrary.Array_Length` (`self.FiringModes`)) 1))
      (set `self.CurrentFiringMode` (`|GetArrayItem` (`self.FiringModes`)))
      (set `self.CurrentFiringModeIndex` 0)
      (else
        (bind _result (`/Engine/EditorBlueprintResources/StandardMacros.IncrementInt` (`self.CurrentFiringModeIndex`))
          (:`  `
            (bind _output_get (set `self.CurrentFiringModeIndex` _result))
            (set `self.CurrentFiringMode` (`|GetArrayItem` (`self.FiringModes`) _output_get))))))
    (`KismetSystemLibrary.PrintString` (`|GetEnumeratorNameAsString` (`self.CurrentFiringMode`)))
    (else
      (`KismetSystemLibrary.PrintString` "GUN HAS NO FIRING MODE" true true (struct :`R` 1.0 :`B` 0.00343 :`A` 1.0)))))

(fn `UserConstructionScript`)